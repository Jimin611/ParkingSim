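; BP_QuestsSaveObject is a save data object that, despite its quest-related name, holds player progression: level, gold, experience and needed experience.
; SaveExpGold copies the passed values into the object's Saved variables, and LoadExpGold returns them.
; It only stores values in memory, with no slot read or write and no quest data in its graphs.
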(fn `LoadExpGold`
  (returns (SavedLevel :type Integer) (SavedGold :type Integer) (SavedExperience :type "Float (double-precision)") (SavedNeededExperience :type "Float (double-precision)"))
  (return (`self.SavedLevel`) (`self.SavedGold`) (`self.SavedExperience`) (`self.SavedNeededExperience`)))

(fn `SaveExpGold`
  (params (Level :type Integer) (Gold :type Integer) (Experience :type "Float (double-precision)") (NeededExperience :type "Float (double-precision)"))
  (set `self.SavedLevel` Level)
  (set `self.SavedGold` (`local.Gold`))
  (set `self.SavedExperience` (`local.Experience`))
  (set `self.SavedNeededExperience` (`local.NeededExperience`)))